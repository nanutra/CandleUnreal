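; BP_CandleStick is a candle that can be lit or unlit, toggling its point light, fire visibility and mesh shadow through SetEnabled, also run at construction.
; When enabled, Tick ramps light intensity up to a threshold, above which the Candleflame timeline animates it between minimum and maximum values.
; When disabled, Tick holds intensity at zero.
; Overlap events track whether the FirstPersonCharacter is nearby, though nothing here reads that flag.
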(event EventBeginPlay
  (bind _intensity (Timeline|Candleflame Play)
    (:Update
      ;[1 1 1] light animation
      (Math|Float|CompareFloat (Variables|/Script/Engine.LightComponentBase|GetIntensity (Variables|Default|GetPointLight)) 4e+03
        (:>
          (Rendering|Components|Light|SetIntensity (Variables|Default|GetPointLight) (Math|Float|Lerp (Variables|Default|GetMaxIntensity) (Variables|Default|GetMinIntensity) _intensity)))))))

(event EventTick
  (params (DeltaSeconds :type Float%20%28single-precision%29))
  (bind _pointlight (Variables|Default|GetPointLight))
  (if (Variables|Default|GetEnabled)
    (Math|Float|CompareFloat (Variables|/Script/Engine.LightComponentBase|GetIntensity _pointlight) 4e+03
      (:<
        (Rendering|Components|Light|SetIntensity _pointlight (+ (Variables|/Script/Engine.LightComponentBase|GetIntensity _pointlight) 1e+01))))
    (else
      (Rendering|Components|Light|SetIntensity (Variables|Default|GetPointLight) 0.0))))

(event Collision|EventActorBeginOverlap
  (params (OtherActor :type Actor%20Object%20Reference))
  (Utilities|Casting|CastToFirstPersonCharacter OtherActor)
  (Variables|Default|SetoverlapPlayer true))

(event Collision|EventActorEndOverlap
  (params (OtherActor :type Actor%20Object%20Reference))
  (Utilities|Casting|CastToFirstPersonCharacter OtherActor)
  (Variables|Default|SetoverlapPlayer false))

(fn ConstructionScript
  (CallFunction|SetEnabled (Variables|Default|GetEnabled)))

(fn SetEnabled
  (params (Enabled :type Boolean))
  (bind _output_get (Variables|Default|SetEnabled Enabled))
  (Rendering|SetVisibility (Variables|Default|GetPointLight) _output_get false)
  (Rendering|SetVisibility (Variables|Default|Getfire) _output_get false)
  (Rendering|SetCastShadow (Variables|Debug|GetStaticMeshComponent) (not _output_get)))