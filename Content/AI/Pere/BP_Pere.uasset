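; BP_Pere is the dad AI actor's Blueprint, which drives his footstep audio from movement speed.
; Each Tick sums absolute X and Y velocity, playing the FootStepsDad sound at a higher pitch above a speed threshold and stopping it at zero.
; A FootStepsPlaying flag prevents restarts, so pitch is set only when playback begins and stays unchanged until he stops.
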(event EventTick
  (params (DeltaSeconds :type Float%20%28single-precision%29))
  (bind _returnvalue (Transformation|GetVelocity))
  (bind _returnvalue_2 (Transformation|GetVelocity))
  (bind _footstepsdad (Variables|Default|GetFootStepsDad))
  (bind (_x _y) (Math|Vector|BreakVector _returnvalue_2))
  (bind (_x_2 _y_2) (Math|Vector|BreakVector _returnvalue))
  ;[0 0.6771 1] FootstepsDad
  (Math|Float|CompareFloat (+ (Math|Float|Absolute(Float) _x_2) (Math|Float|Absolute(Float) _y_2)) 0.0
    (:>
      (Math|Float|CompareFloat (+ (Math|Float|Absolute(Float) _x) (Math|Float|Absolute(Float) _y)) 3e+02
        (:>
          (if (not (Variables|Default|GetFootStepsPlaying))
            (Audio|Components|Audio|SetPitchMultiplier _footstepsdad 2.0)
            (Audio|Components|Audio|Play _footstepsdad 0.0)
            (Variables|Default|SetFootStepsPlaying true)))
        (:==
          (if (not (Variables|Default|GetFootStepsPlaying)) :!label _label
            (Audio|Components|Audio|SetPitchMultiplier _footstepsdad 1.2)
            (Audio|Components|Audio|Play _footstepsdad 0.0)
            (Variables|Default|SetFootStepsPlaying true)))
        (:<
          (goto _label))))
    (:==
      (Variables|Default|SetFootStepsPlaying false)
      (Audio|Components|Audio|Stop (Variables|Default|GetFootStepsDad)))))

(fn ConstructionScript)