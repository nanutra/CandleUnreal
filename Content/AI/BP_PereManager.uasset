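; Manager that stages the encounters with the Père AI variants: Tuto, Roaming, Chase, Fauteuil and EnigmeFin.
; Player-triggered overlap volumes teleport pre-placed AIs between standby and spawn points, destroying Roaming and Fauteuil as later chases begin.
; Player death delegates, bound after a BeginPlay delay, return the relevant AI to standby, or restart the level for Tuto.
; Fauteuil death also clears its IsSpawned blackboard key and resets the window and fire.
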(event OnComponentBeginOverlap(TriggerRoaming)
  (params (OverlappedComponent :type Primitive%20Component%20Object%20Reference) (OtherActor :type Actor%20Object%20Reference) (OtherComp :type Primitive%20Component%20Object%20Reference) (OtherBodyIndex :type Integer) (bFromSweep :type Boolean) (SweepResult :type Hit%20Result%20Structure%20%28by%20ref%29))
  (bind _pereroamingref (Variables|Default|GetPereRoamingRef))
  (bind _output (Utilities|ResolveSoftReference _pereroamingref))
  ;[0.1253 0.1005 1] TriggerRoaming
  (if (not (Variables|Default|GetRoamingTriggered?))
    (Utilities|Casting|CastToBP_Player OtherActor)
    (if (Utilities|IsValid _output)
      (Transformation|SetActorLocation _output (Transformation|GetWorldLocation (Variables|Default|GetSpawnPereRoaming)) false true)
      (Variables|Default|SetRoamingTriggered? true)
      (else
        (Development|PrintString "PereRoaming n'éxiste plus")))))

(event OnComponentBeginOverlap(TriggerChase)
  (params (OverlappedComponent :type Primitive%20Component%20Object%20Reference) (OtherActor :type Actor%20Object%20Reference) (OtherComp :type Primitive%20Component%20Object%20Reference) (OtherBodyIndex :type Integer) (bFromSweep :type Boolean) (SweepResult :type Hit%20Result%20Structure%20%28by%20ref%29))
  (bind _perechaseref (Variables|Default|GetPereChaseRef))
  (bind _pereroamingref (Variables|Default|GetPereRoamingRef))
  (bind _output (Utilities|ResolveSoftReference _perechaseref))
  (bind _output_2 (Utilities|ResolveSoftReference _pereroamingref))
  ;[1 0.124 0.1638] TriggerChase
  (Utilities|Casting|CastToBP_Player OtherActor)
  (if (Utilities|IsValid _output)
    (Transformation|SetActorLocation _output (Transformation|GetWorldLocation (Variables|Default|GetSpawnPereChase)) false true)
    (if (Utilities|IsValid _output_2)
      (Actor|DestroyActor _output_2))))

(event OnComponentBeginOverlap(StopChase)
  (params (OverlappedComponent :type Primitive%20Component%20Object%20Reference) (OtherActor :type Actor%20Object%20Reference) (OtherComp :type Primitive%20Component%20Object%20Reference) (OtherBodyIndex :type Integer) (bFromSweep :type Boolean) (SweepResult :type Hit%20Result%20Structure%20%28by%20ref%29))
  (bind _perefauteuilref (Variables|Default|GetPereFauteuilRef))
  (bind _perefauteuilref_2 (Variables|Default|GetPereFauteuilRef))
  (bind _perechaseref (Variables|Default|GetPereChaseRef))
  (bind _output (Utilities|ResolveSoftReference _perechaseref))
  (bind _output_2 (Utilities|ResolveSoftReference _perefauteuilref))
  (bind _output_3 (Utilities|ResolveSoftReference _perefauteuilref_2))
  ;[0 0 0] DespawnPereChase / SpawnPereFauteuil
  (Utilities|Casting|CastToBP_Player OtherActor)
  (if (Utilities|IsValid _output)
    (Transformation|SetActorLocation _output (Transformation|GetWorldLocation (Variables|Default|GetPereChaseStandBy)) false true)
    (if (Utilities|IsValid _output_3)
      (Transformation|SetActorLocation _output_3 (Transformation|GetWorldLocation (Variables|Default|GetSpawnPereFauteuil)) false true)
      (Variables|Default|SetIsSpawned true)
      (AI|Components|Blackboard|SetValueasBool (Variables|/Script/AIModule.AIController|GetBlackboard (AI|GetAIController _output_3)) (Utilities|Name|MakeLiteralName "IsSpawned") true)
      (Transformation|SetActorRotation _output_2 (Math|Rotator|FindLookatRotation (Pawn|GetNavAgentLocation _output_2) (Transformation|GetWorldLocation (Variables|Default|GetLookAtComponent)))))))

(event OnComponentBeginOverlap(TriggerChase2)
  (params (OverlappedComponent :type Primitive%20Component%20Object%20Reference) (OtherActor :type Actor%20Object%20Reference) (OtherComp :type Primitive%20Component%20Object%20Reference) (OtherBodyIndex :type Integer) (bFromSweep :type Boolean) (SweepResult :type Hit%20Result%20Structure%20%28by%20ref%29))
  (bind _perefauteuilref (Variables|Default|GetPereFauteuilRef))
  (bind _perechaseref (Variables|Default|GetPereChaseRef))
  (bind _output (Utilities|ResolveSoftReference _perefauteuilref))
  (bind _output_2 (Utilities|ResolveSoftReference _perechaseref))
  ;[1 0.02083 0.02083] SpawnChase2
  (Utilities|Casting|CastToBP_Player OtherActor)
  (if (Utilities|IsValid _output_2)
    (Transformation|SetActorLocation _output_2 (Transformation|GetWorldLocation (Variables|Default|GetSpawnPereChase2)) false true)
    (if (Utilities|IsValid _output)
      (Actor|DestroyActor _output))))

(event OnComponentBeginOverlap(StopChase2)
  (params (OverlappedComponent :type Primitive%20Component%20Object%20Reference) (OtherActor :type Actor%20Object%20Reference) (OtherComp :type Primitive%20Component%20Object%20Reference) (OtherBodyIndex :type Integer) (bFromSweep :type Boolean) (SweepResult :type Hit%20Result%20Structure%20%28by%20ref%29))
  (bind _perechaseref (Variables|Default|GetPereChaseRef))
  (bind _output (Utilities|ResolveSoftReference _perechaseref))
  ;[0.08683 1 0.1237] StopChase2/SpawnEnigmeFin
  (Utilities|Casting|CastToBP_Player OtherActor)
  (if (Utilities|IsValid _output)
    (Transformation|SetActorLocation _output (Transformation|GetWorldLocation (Variables|Default|GetPereChaseStandBy)) false true)
    (Transformation|SetActorLocation (Utilities|ResolveSoftReference (Variables|Default|GetPereEnigmeFinRef)) (Transformation|GetWorldLocation (Variables|Default|GetSpawnPereEnigmeFin)) false true)))

(event Custom|Died%20%28%20EnigmeFin%20%29
  ;[1 0.103 0.0831] DiedToPereEnigmeFin
  (Utilities|Casting|CastToIA_Pere_EnigmeFin (AI|GetAIController (Utilities|ResolveSoftReference (Variables|Default|GetPereEnigmeFinRef))))
  (Default|CallResetPereEnigmeFin)
  (Transformation|SetActorLocation (Transformation|GetWorldLocation (Variables|Default|GetPereEnigmeFinStandBy)) false true))

(event Custom|Died%20%28Chase%29
  ;[1 0.1238 0.1039] DiedToPereChase
  (Transformation|SetActorLocation (Utilities|ResolveSoftReference (Variables|Default|GetPereChaseRef)) (Transformation|GetWorldLocation (Variables|Default|GetPereChaseStandBy)) false true))

(event Custom|Died%20%28Roaming%29
  ;[1 0.125 0.125] DiedToPereRoaming
  (Transformation|SetActorLocation (Utilities|ResolveSoftReference (Variables|Default|GetPereRoamingRef)) (Transformation|GetWorldLocation (Variables|Default|GetPereRoamingStandBy)) false true))

(event Custom|Died%20%28Fauteuil%29
  (bind _perefauteuilref (Variables|Default|GetPereFauteuilRef))
  (bind _output (Utilities|ResolveSoftReference _perefauteuilref))
  ;[1 0.103 0.0831] DiedToPereFauteuil
  (Transformation|SetActorLocation _output (Transformation|GetWorldLocation (Variables|Default|GetPereFauteuilStandBy)) false true)
  (AI|Components|Blackboard|SetValueasBool (Variables|/Script/AIModule.AIController|GetBlackboard (AI|GetAIController _output)) (Utilities|Name|MakeLiteralName "IsSpawned") false)
  (if (Variables|/Game/BluePrint/Iteractibles/Window.Window_C|GetIsWindowOpen (Utilities|ResolveSoftReference (Variables|Default|GetWindowRef)))
    (Default|CallResetWindow))
  (if (Variables|/Game/BluePrint/DadInteractions/BP_FeuDeCheminée.BP_FeuDeCheminée_C|GetIsFireOn? (Utilities|ResolveSoftReference (Variables|Default|GetFireRef)))
    (Default|CallResetFire)))

(event Custom|Died%20%28Tuto%29
  ;[1 0.103 0.0831] DiedToPereEnigmeFin
  (Default|CallRestartLevel))

(event EventBeginPlay
  (Utilities|FlowControl|Delay 3.0)
  (Transformation|SetActorLocation (Utilities|ResolveSoftReference (Variables|Default|GetPereTutoRef)) (Transformation|GetWorldLocation (Variables|Default|GetSpawnPereTuto)) false true)
  (bind _asbp_player (Utilities|Casting|CastToBP_Player (Game|Player|GetPlayerPawn 0)))
  ;[1 0.125 0.125] DiedToPereRoaming
  (EventDispatchers|BindEventtoDiedtoPere _asbp_player (delegate Custom|Died%20%28Roaming%29))
  ;[1 0.1238 0.1039] DiedToPereChase
  (EventDispatchers|BindEventtoDiedtoPereChase _asbp_player (delegate Custom|Died%20%28Chase%29))
  ;[1 0.103 0.0831] DiedToPereFauteuil
  (EventDispatchers|BindEventtoDiedtoPereFauteuil _asbp_player (delegate Custom|Died%20%28Fauteuil%29))
  ;[1 0.103 0.0831] DiedToPereEnigmeFin
  (EventDispatchers|BindEventtoDiedtoPereTuto _asbp_player (delegate Custom|Died%20%28Tuto%29))
  ;[1 0.103 0.0831] DiedToPereEnigmeFin
  (EventDispatchers|BindEventtoDiedtoPereEnigmeFin _asbp_player (delegate Custom|Died%20%28%20EnigmeFin%20%29)))

(fn ConstructionScript)