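; End-of-game door that triggers the ending when a player holding the key overlaps it.
; It disables the player's movement and saves the first-person camera's location as the cinematic location.
; One timeline swings the Plane mesh slightly open, then after a pause a second timeline swings it back.
; After a final short delay, it calls the player's StartEndScene.
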(event Collision|EventActorBeginOverlap
  (params (OtherActor :type Actor%20Object%20Reference))
  (bind _asbp_player (Utilities|Casting|CastToBP_Player OtherActor))
  (if (Variables|/Game/BluePrint/Players_BP/BP_Player.BP_Player_C|GetHaveKey _asbp_player)
    (Variables|/Game/BluePrint/Players_BP/BP_Player.BP_Player_C|SetCanMove _asbp_player false)
    (Variables|/Game/BluePrint/Players_BP/BP_Player.BP_Player_C|SetCineLocation _asbp_player (Transformation|GetWorldLocation (Variables|/Game/BluePrint/Players_BP/BP_Player.BP_Player_C|GetFirstPersonCamera _asbp_player)))
    (bind _ouverture (Timeline|Timeline_0 Play)
      (:Update
        (Transformation|SetRelativeRotation (Variables|Default|GetPlane) (Math|Rotator|Lerp(Rotator) "0, 0, 0" "0,20.000000, 0" _ouverture) false false))
      (:Finished
        (Utilities|FlowControl|Delay 1.0)
        (Utilities|FlowControl|Delay 1.0)
        (bind _fermetire (Timeline|Timeline_1 PlayFromStart)
          (:Update
            (Transformation|SetRelativeRotation (Variables|Default|GetPlane) (Math|Rotator|Lerp(Rotator) "0.000000,20.000000, 0" "0, 0, 0" _fermetire) false false))
          (:Finished
            (bind _asbp_player_2 (Utilities|Casting|CastToBP_Player OtherActor))
            (Utilities|FlowControl|Delay 0.4)
            (Default|StartEndScene _asbp_player_2)))))))

(fn ConstructionScript)