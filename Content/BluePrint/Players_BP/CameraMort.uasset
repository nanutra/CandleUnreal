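; CameraMort is a death camera pawn that briefly takes over the view before the player respawns.
; On possession it turns its camera component toward the stored PerePos location using a look-at rotation.
; After a short delay it hands player controller 0 back to PlayerRef and calls RespawnAfterDeath on it.
; An alternative actor-rotation branch is left unconnected.
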(event EventPossessed
  (params (NewController :type Controller%20Object%20Reference))
  (bind _returnvalue (Transformation|GetActorLocation))
  (bind _perepos (Variables|Default|GetPerePos))
  (bind _returnvalue_2 (Math|Rotator|FindLookatRotation _returnvalue _perepos))
  (bind (_roll _pitch _yaw) (Math|Rotator|BreakRotator _returnvalue_2))
  (Transformation|SetRelativeRotation (Variables|Default|GetCamera) (Math|Rotator|MakeRotator _roll _pitch _yaw) false false)
  (Utilities|FlowControl|Delay 4.0)
  (Pawn|Possess (Game|GetPlayerController 0) (Variables|Default|GetPlayerRef))
  (Default|RespawnAfterDeath (Variables|Default|GetPlayerRef)))

(fn ConstructionScript)