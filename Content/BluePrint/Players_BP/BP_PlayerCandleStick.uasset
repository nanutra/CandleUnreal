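; BP_PlayerCandleStick is a candlestick, apparently carried by the player, with a flickering point light and a fire effect that can be switched on or off.
; On BeginPlay, the Candleflame timeline drives the light intensity between its max and min values.
; SetEnabled, also run from the construction script, toggles light and fire visibility and makes the mesh cast shadows only when unlit.
; The GetPosForFlame event is an empty stub.
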(event Custom|GetPosForFlame
  (params (NewParam :type Vector)))

(event EventBeginPlay
  (bind _intensity (Timeline|Candleflame Play)
    (:Update
      (Rendering|Components|Light|SetIntensity (Variables|Default|GetPointLight) (Math|Float|Lerp (Variables|Default|GetMaxIntensity) (Variables|Default|GetMinIntensity) _intensity)))))

(fn ConstructionScript
  (CallFunction|SetEnabled (Variables|Default|GetEnabled)))

(fn SetEnabled
  (params (Enabled :type Boolean))
  (bind _output_get (Variables|Default|SetEnabled Enabled))
  (Rendering|SetVisibility (Variables|Default|GetPointLight) _output_get false)
  (Rendering|SetVisibility (Variables|Default|Getfire) _output_get false)
  (Rendering|SetCastShadow (Variables|Debug|GetStaticMeshComponent) (not _output_get)))