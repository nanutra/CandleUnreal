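; Chained camera pawn for what appears to be a tutorial intro sequence, flagged as first, middle or last link.
; The first link possesses the player controller on BeginPlay and starts an eased view-target blend to NextCam.
; Each middle link's Transi waits, toggles its collision, then triggers and blends to the next.
; The last link teleports PlayerRef to InitPosePlayer, resets its Stress and hands possession back to it.
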(event Custom|Transi
  (bind _returnvalue (Game|GetPlayerController 0))
  (bind _nextcam (Variables|Default|GetNextCam))
  (bind _playerref (Variables|Default|GetPlayerRef))
  (Utilities|FlowControl|Delay 1.0)
  (if (not (Variables|Default|GetisFirst))
    (if (Variables|Default|GetIsLast)
      (Utilities|FlowControl|Delay 1.0)
      (Transformation|SetWorldLocation (Variables|/Script/Engine.Actor|GetRootComponent _playerref) (Variables|Default|GetInitPosePlayer) false true)
      (Collision|SetActorEnableCollision false)
      (Collision|SetActorEnableCollision true)
      (Variables|/Game/BluePrint/Players_BP/BP_Player.BP_Player_C|SetStress _playerref 0.0)
      (Pawn|Possess _returnvalue _playerref)
      (else
        (Utilities|FlowControl|Delay 2.0)
        (Collision|SetActorEnableCollision false)
        (Collision|SetActorEnableCollision true)
        (CallFunction|Transi _nextcam)
        (Game|Player|SetViewTargetwithBlend _returnvalue _nextcam 2.0 "VTBlend_EaseInOut" 2.0 false)))))

(event EventBeginPlay
  (bind _returnvalue (Game|GetPlayerController 0))
  (bind _nextcam (Variables|Default|GetNextCam))
  (if (Variables|Default|GetisFirst)
    (Pawn|Possess _returnvalue self)
    (Collision|SetActorEnableCollision false)
    (Collision|SetActorEnableCollision true)
    (CallFunction|Transi _nextcam)
    (Game|Player|SetViewTargetwithBlend _returnvalue _nextcam 2.0 "VTBlend_EaseInOut" 2.0 false)))

(fn ConstructionScript)