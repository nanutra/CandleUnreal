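; BP_PortesEnfants is a trigger actor for a pair of doors, built from two planes that rotate when an actor overlaps it.
; BeginPlay sets each plane to its own start rotation, then the overlap plays a timeline that lerps both from those rotations toward a zero rotation.
; When the timeline finishes, it sets a one-time sound-played flag if sound is allowed, though no sound is played here.
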(event Collision|EventActorBeginOverlap
  (params (OtherActor :type Actor%20Object%20Reference))
  (bind _rotation (Timeline|Timeline_0 Play)
    (:Update
      (Transformation|SetRelativeRotation (Variables|Default|GetPlane1) (Math|Rotator|Lerp(Rotator) (Variables|Default|GetStartRotaDoor1) "0, 0, 0" _rotation) false false)
      (Transformation|SetRelativeRotation (Variables|Default|GetPlane2) (Math|Rotator|Lerp(Rotator) (Variables|Default|GetStartRotaDoor2) "0, 0, 0" _rotation) false false))
    (:Finished
      (if (Variables|Default|GetCanPlaySound)
        (if (not (Variables|Default|GetSoundIsPlayed))
          (Variables|Default|SetSoundIsPlayed true))))))

(event EventBeginPlay
  (Transformation|SetRelativeRotation (Variables|Default|GetPlane1) (Variables|Default|GetStartRotaDoor1) false false)
  (Transformation|SetRelativeRotation (Variables|Default|GetPlane2) (Variables|Default|GetStartRotaDoor2) false false))

(fn ConstructionScript)