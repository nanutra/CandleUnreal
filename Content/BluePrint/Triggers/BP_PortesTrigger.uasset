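; BP_PortesTrigger is a trigger actor that opens doors when the player overlaps it.
; On overlap with BP_Player, a DoTuto flag selects either the tutorial door list or the regular door list and calls OpenDoor on each entry.
; Each opened door also prints a "Hello" debug string, and an unconnected branch reading an AI controller countdown never runs.
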(event Collision|EventActorBeginOverlap
  (params (OtherActor :type Actor%20Object%20Reference))
  (Utilities|Casting|CastToBP_Player OtherActor)
  (if (Variables|Default|GetdoTuto)
    (for _array_element (Variables|Default|GetDoorTutoList)
      (Default|OpenDoor _array_element)
      (Development|PrintString "Hello"))
    (else
      (for _array_element_2 (Variables|Default|GetDoorsList)
        (Default|OpenDoor _array_element_2)
        (Development|PrintString "Hello")))))

(fn ConstructionScript)