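; Interactable window jump scare that swings open when the player walks into it and can then be closed.
; The first overlap plays a timeline rotating two mirrored panels open, enables interaction and, after a short delay, calls WindTurnOff on the player.
; Later overlaps only repeat that player call.
; Interagir, once enabled, or ClosingScreamer plays a second timeline that rotates the panels back.
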(event Custom|ClosingScreamer
  ;[1 1 1] rotation animation
  (bind _rotation (Timeline|Timeline_1 Play)
    (:Update
      (Transformation|SetRelativeRotation (Variables|Default|Getrota1) (Class|KismetMathLibrary|NegateRotator (Math|Rotator|Lerp(Rotator) (Variables|Default|GetendRota) (Variables|Default|GetstartRota) _rotation)) false false)
      (Transformation|SetRelativeRotation (Variables|Default|Getrota2) (Math|Rotator|Lerp(Rotator) (Variables|Default|GetendRota) (Variables|Default|GetstartRota) _rotation) false false))))

(event Collision|EventActorBeginOverlap
  (params (OtherActor :type Actor%20Object%20Reference))
  (bind _asbp_player (Utilities|Casting|CastToBP_Player OtherActor))
  (if (Variables|Default|GetbeenActivated)
    (Default|WindTurnOff _asbp_player)
    (else
      (bind _rotation (Timeline|Timeline_0 Play)
        (:Update
          (Transformation|SetRelativeRotation (Variables|Default|Getrota1) (Class|KismetMathLibrary|NegateRotator (Math|Rotator|Lerp(Rotator) (Variables|Default|GetstartRota) (Variables|Default|GetendRota) _rotation)) false false)
          (Transformation|SetRelativeRotation (Variables|Default|Getrota2) (Math|Rotator|Lerp(Rotator) (Variables|Default|GetstartRota) (Variables|Default|GetendRota) _rotation) false false)
          (Variables|Default|SetbeenActivated true)
          (Variables|Default|SetcanInteract true)
          (Utilities|FlowControl|Delay 0.1)
          (Default|WindTurnOff _asbp_player))))))

(event EventInteragir
  (if (Variables|Default|GetcanInteract)
    ;[1 1 1] rotation animation
    (bind _rotation (Timeline|Timeline_1 Play)
      (:Update
        (Transformation|SetRelativeRotation (Variables|Default|Getrota1) (Class|KismetMathLibrary|NegateRotator (Math|Rotator|Lerp(Rotator) (Variables|Default|GetendRota) (Variables|Default|GetstartRota) _rotation)) false false)
        (Transformation|SetRelativeRotation (Variables|Default|Getrota2) (Math|Rotator|Lerp(Rotator) (Variables|Default|GetendRota) (Variables|Default|GetstartRota) _rotation) false false)))))

(fn ConstructionScript
  (|CallParentFunction))

(fn Closing)