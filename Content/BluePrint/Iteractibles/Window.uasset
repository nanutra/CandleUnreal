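; Interactable window with two mirrored shutters or panes that the player opens, notifying the father character (BP_PereFauteil) of its state.
; Interacting clears the custom-depth highlight, plays the opening sound, raises the storm volume and swings both sides open through a timeline.
; The father overlapping the box, or a reset event bound through the father manager, reports it closed and swings it shut after a short delay.
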(event OnComponentBeginOverlap(Box)
  (params (OverlappedComponent :type Primitive%20Component%20Object%20Reference) (OtherActor :type Actor%20Object%20Reference) (OtherComp :type Primitive%20Component%20Object%20Reference) (OtherBodyIndex :type Integer) (bFromSweep :type Boolean) (SweepResult :type Hit%20Result%20Structure%20%28by%20ref%29))
  ;[0.9909 1 0] OverlapPere
  (bind _asbp_pere_fauteil (Utilities|Casting|CastToBP_PereFauteil OtherActor))
  (CallFunction|Closing _asbp_pere_fauteil))

(event Custom|Closing
  (params (PereFauteuil :type BP%20Pere%20Fauteil%20Object%20Reference))
  ;[1 0 0.08657] ClosingFunction
  (Class|BPInterfaceIA|WindowOpen(Message) PereFauteuil false)
  (Variables|Default|SetIsWindowOpen false)
  (Utilities|FlowControl|Delay 1.0)
  (bind _rotation (Timeline|Timeline_1 Play)
    (:Update
      (Transformation|SetRelativeRotation (Variables|Default|Getrota3) (Class|KismetMathLibrary|NegateRotator (Math|Rotator|Lerp(Rotator) (Variables|Default|GetendRota) (Variables|Default|GetstartRota) _rotation)) false false)
      (Transformation|SetRelativeRotation (Variables|Default|Getrota4) (Math|Rotator|Lerp(Rotator) (Variables|Default|GetendRota) (Variables|Default|GetstartRota) _rotation) false false))))

(event Custom|CloseWindow
  ;[1 1 1] ResetWindow
  (bind _asbp_pere_fauteil (Utilities|Casting|CastToBP_PereFauteil (Variables|Default|GetPereSoftRef)))
  (CallFunction|Closing _asbp_pere_fauteil))

(event EventBeginPlay
  (Rendering|SetRenderCustomDepth (Variables|Default|GetCube1) true)
  (Rendering|SetCustomDepthStencilValue (Variables|Default|GetCube2) 1)
  ;[0 0.9482 1] SoundInitialization
  (Audio|Components|Audio|SetVolumeMultiplier (Variables|Default|GetStormSound) 0.08 :!class /Script/Engine.AudioComponent)
  ;[1 1 1] ResetWindow
  (EventDispatchers|BindEventtoResetWindow (Utilities|ResolveSoftReference (Variables|Default|GetBP_PereManagerRef)) (delegate Custom|CloseWindow)))

(event EventInteragir
  (Rendering|SetRenderCustomDepth (Variables|Default|GetCube1) false)
  (if (Variables|Default|GetcanOpen)
    (Variables|Default|SetcanOpen false)
    ;[0 0.9482 1] SoundInitialization
    (Audio|Components|Audio|Play (Variables|Default|GetWindowOpenSound) 0.2)
    (Audio|Components|Audio|SetVolumeMultiplier (Variables|Default|GetStormSound) 0.5 :!class /Script/Engine.AudioComponent)
    ;[1 1 1] rotation animation
    (bind _rotation (Timeline|rotaton Play)
      (:Update
        (Transformation|SetRelativeRotation (Variables|Default|Getrota3) (Class|KismetMathLibrary|NegateRotator (Math|Rotator|Lerp(Rotator) (Variables|Default|GetstartRota) (Variables|Default|GetendRota) _rotation)) false false)
        (Transformation|SetRelativeRotation (Variables|Default|Getrota4) (Math|Rotator|Lerp(Rotator) (Variables|Default|GetstartRota) (Variables|Default|GetendRota) _rotation) false false)
        (bind _asbp_pere_fauteil (Utilities|Casting|CastToBP_PereFauteil (Variables|Default|GetPereSoftRef)))
        (Class|BPInterfaceIA|WindowOpen(Message) _asbp_pere_fauteil true)
        (Variables|Default|SetIsWindowOpen true))
      (:Finished
        (Variables|Default|SetcanOpen true)))))

(fn ConstructionScript
  (|CallParentFunction))

(fn OpenWindow
  (bind _startrota (Variables|Default|GetstartRota))
  (bind _endrota (Variables|Default|GetendRota))
  (bind _returnvalue (Math|Rotator|Lerp(Rotator) _startrota _endrota 0.0))
  (Transformation|SetRelativeRotation (Variables|Default|Getrota3) (Class|KismetMathLibrary|NegateRotator _returnvalue) false false)
  (Transformation|SetRelativeRotation (Variables|Default|Getrota4) _returnvalue false false)
  (return))