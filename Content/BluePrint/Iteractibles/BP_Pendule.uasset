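; Interactable pendulum clock that can be activated once through Interagir, which sets IsUsed and calls OnObjectActivated.
; While unused, Tick plays the ColorLerp timeline, which drives a material parameter on the clock mesh and creates a dynamic material instance every update.
; The timeline restarts itself on finish without checking IsUsed, so the color pulse keeps looping after use.
; CompareDistance is an unfinished, debug-print player proximity check that is never called.
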(event EventBeginPlay)

(event Collision|EventActorBeginOverlap
  (params (OtherActor :type Actor%20Object%20Reference))
  (|CallParentFunction OtherActor) ; This node is disabled and will not be called.\nDrag off pins to build functionality.
)

(event EventTick
  (params (DeltaSeconds :type Float%20%28single-precision%29))
  (if (not (Variables|Default|GetIsUsed))
    (bind _newtrack_0 (Timeline|ColorLerp Play)
      (:Update
        (bind _returnvalue (Rendering|Material|CreateDynamicMaterialInstance (Variables|Default|GetHorlogeUvsFM) 0 0 "None" :!class /Script/Engine.PrimitiveComponent))
        (Rendering|Material|SetScalarParameterValue _returnvalue "ColorLerp" _newtrack_0 :!class /Script/Engine.MaterialInstanceDynamic))
      (:Finished
        (Variables|Default|SetIsUsed (Variables|Default|GetIsUsed))
        (Timeline|ColorLerp PlayFromStart)))))

(event EventInteragir
  (if (not (Variables|Default|GetIsUsed))
    (Variables|Default|SetIsUsed true)
    (Default|CallOnObjectActivated)
    (Development|PrintString "Penduleu")))

(fn ConstructionScript
  (|CallParentFunction))

(fn CompareDistance
  (bind _returnvalue (Game|GetPlayerController 0))
  (bind _horlogeuvsfm (Variables|Default|GetHorlogeUvsFM))
  (bind _returnvalue_2 (Transformation|GetWorldLocation _horlogeuvsfm))
  (bind _rootcomponent (Variables|/Script/Engine.Actor|GetRootComponent _returnvalue))
  (bind (_x _y) (Math|Vector|BreakVector _returnvalue_2))
  (bind _returnvalue_3 (Transformation|GetWorldLocation _rootcomponent))
  (bind (_x_2 _y_2) (Math|Vector|BreakVector _returnvalue_3))
  (bind _returnvalue_4 (- _x_2 _x))
  (Development|PrintString (Utilities|String|ToString(Float) _returnvalue_4))
  (Math|Float|CompareFloat _returnvalue_4 (* (Variables|Default|GetDistance) -1.0)
    (:>
      (Development|PrintString "Hello")
      (return))))