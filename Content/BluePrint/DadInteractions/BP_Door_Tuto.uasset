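; BP_Door_Tuto is a double door, likely for the tutorial, built from two planes that can swing open or be broken.
; BeginPlay gives the planes mirrored starting rotations and stops both door sounds.
; OpenDoor plays the open sound while a timeline lerps the planes toward mirrored end rotations.
; BreakDoor uses a second timeline to rotate both planes to one shared broken rotation, without sound.
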(event Custom|OpenDoor
  (Audio|Components|Audio|Play (Variables|Default|GetOpenDoorSound) 0.0)
  (bind _rotation (Timeline|Timeline_0 Play)
    (:Update
      (Transformation|SetRelativeRotation (Variables|Default|GetPlane) (Math|Rotator|Lerp(Rotator) (Variables|Default|GetstartRota) (Variables|Default|GetendRota) _rotation) false false)
      (Transformation|SetRelativeRotation (Variables|Default|GetPlane2) (Math|Rotator|Lerp(Rotator) (Variables|Default|GetstartRota) (Class|KismetMathLibrary|NegateRotator (Variables|Default|GetendRota)) _rotation) false false))))

(event Custom|BreakDoor
  (bind _rotation (Timeline|Timeline_1 Play)
    (:Update
      (Transformation|SetRelativeRotation (Variables|Default|GetPlane) (Math|Rotator|Lerp(Rotator) "0,90.000000, 0" (Variables|Default|GetvectorBreakDoor) _rotation) false false)
      (Transformation|SetRelativeRotation (Variables|Default|GetPlane2) (Math|Rotator|Lerp(Rotator) "0,90.000000, 0" (Variables|Default|GetvectorBreakDoor) _rotation) false false))))

(event EventBeginPlay
  (Transformation|SetRelativeRotation (Variables|Default|GetPlane) (Variables|Default|GetNewRota) false false)
  (Audio|Components|Audio|Stop (Variables|Default|GetOpenDoorSound))
  (Transformation|SetRelativeRotation (Variables|Default|GetPlane2) (Class|KismetMathLibrary|NegateRotator (Variables|Default|GetNewRota)) false false))

(fn ConstructionScript)