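; BP_FeuDeCheminée is a fireplace actor that shows a Niagara fire and point light, switched on at BeginPlay.
; A ResetIntensity event turns off the light, hides the fire and clears IsFireOn, with a debug print.
; The trigger overlap is empty; delayed lighting by BP_PereFauteil and binding the reset to the father manager sit in disconnected nodes.
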(event OnComponentBeginOverlap(FireTrigger)
  (params (OverlappedComponent :type Primitive%20Component%20Object%20Reference) (OtherActor :type Actor%20Object%20Reference) (OtherComp :type Primitive%20Component%20Object%20Reference) (OtherBodyIndex :type Integer) (bFromSweep :type Boolean) (SweepResult :type Hit%20Result%20Structure%20%28by%20ref%29)))

(event Custom|ResetIntensity
  ;[1 0.7523 0.09375] ResetFire
  (Development|PrintString "ZQFQDZ")
  (Rendering|Components|Light|SetIntensity (Variables|Default|GetPointLight) 0.0)
  (Rendering|SetVisibility (Variables|Default|GetNS_fire) false false)
  (Variables|Default|SetIsFireOn? false))

(event EventBeginPlay
  (Rendering|SetVisibility (Variables|Default|GetNS_fire) true false)
  (Rendering|Components|Light|SetIntensity (Variables|Default|GetPointLight) 5e+03))

(fn ConstructionScript)