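; Falling furniture actor that tips its Plane component over by 90 degrees when another actor overlaps it.
; An overlap plays a timeline that lerps the Plane's relative rotation, without filtering the overlapping actor.
; When the timeline finishes, it triggers a camera shake if that actor is BP_Player.
; Fall and Reset functions snap the rotation to fallen or upright, but the event graph's Fall call is unconnected.
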(event EventBeginPlay)

(event Collision|EventActorBeginOverlap
  (params (OtherActor :type Actor%20Object%20Reference))
  (bind _newtrack_0 (Timeline|Timeline_0 Play)
    (:Update
      _)
    (:Finished
      (bind _asbp_player (Utilities|Casting|CastToBP_Player OtherActor))
      (Default|CameraShake _asbp_player)))
  (Transformation|SetRelativeRotation (Variables|Default|GetPlane) (Math|Rotator|Lerp(Rotator) "0, 0, 0" "-90.000000, 0, 0" _newtrack_0) false false))

(event EventTick
  (params (DeltaSeconds :type Float%20%28single-precision%29)))

(fn ConstructionScript)

(fn Fall
  (Transformation|SetRelativeRotation (Variables|Default|GetPlane) "-90.000000, 0, 0" false false))

(fn Reset
  (Transformation|SetRelativeRotation (Variables|Default|GetPlane) "0, 0, 0" false false)
  (return))