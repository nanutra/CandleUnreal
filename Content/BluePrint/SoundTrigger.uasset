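; SoundTrigger is a box trigger Blueprint that plays a sound when the player's capsule enters it.
; On BeginPlay it stops the sound and binds a reset to BP_Player's Died event, which sets CanTrigger to true.
; Overlaps are gated by CanTrigger, but playing the sound also sets that flag to true rather than false, so it does not limit playback to once.
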(event OnComponentBeginOverlap(Box)
  (params (OverlappedComponent :type Primitive%20Component%20Object%20Reference) (OtherActor :type Actor%20Object%20Reference) (OtherComp :type Primitive%20Component%20Object%20Reference) (OtherBodyIndex :type Integer) (bFromSweep :type Boolean) (SweepResult :type Hit%20Result%20Structure%20%28by%20ref%29))
  (if (Variables|Default|GetCanTrigger)
    (Utilities|Casting|CastToBP_Player OtherActor)
    (Utilities|Casting|CastToCapsuleComponent OtherComp)
    (Audio|Components|Audio|Play (Variables|Default|GetSoundToTrigger) 0.0)
    (Variables|Default|SetCanTrigger true)))

(event Custom|ResetSoundTrigger
  (Variables|Default|SetCanTrigger true))

(event EventBeginPlay
  (Audio|Components|Audio|Stop (Variables|Default|GetSoundToTrigger))
  (bind _asbp_player (Utilities|Casting|CastToBP_Player (Game|Player|GetPlayerPawn 0)))
  (EventDispatchers|BindEventtoDied _asbp_player (delegate Custom|ResetSoundTrigger)))

(fn ConstructionScript)