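; BP_CandleStick is a candle actor whose light, flame particles and mesh shadow are toggled through SetEnabled.
; When enabled, Tick ramps the point light up to a threshold, above which the Candleflame timeline flickers it.
; SetEnabled takes the timer from the player's candle maximum, and BeginPlay or ChangeAnim passes it to the candle's animation Blueprint.
; Overlap events flag contact with a player whose light is on.
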(event Custom|ChangeAnim
  (bind _asbp_anim_bougie (Utilities|Casting|CastToBP_Anim_Bougie (Components|SkeletalMesh|GetAnimInstance (Variables|Default|GetSkeletalMesh)))
    (:then
      (Variables|/Game/BluePrint/Players_BP/BougieAnim/BP_Anim_Bougie.BP_Anim_Bougie_C|SetTimer _asbp_anim_bougie (Variables|Default|GetCurTimer)))
    (:CastFailed
      (Development|PrintString "failed"))))

(event EventBeginPlay
  (bind _asbp_anim_bougie (Utilities|Casting|CastToBP_Anim_Bougie (Components|SkeletalMesh|GetAnimInstance (Variables|Default|GetSkeletalMesh))))
  (Variables|/Game/BluePrint/Players_BP/BougieAnim/BP_Anim_Bougie.BP_Anim_Bougie_C|SetTimer _asbp_anim_bougie (Variables|Default|GetCurTimer))
  (bind _intensity (Timeline|Candleflame Play)
    (:Update
      ;[1 1 1] light animation
      (Math|Float|CompareFloat (Variables|/Script/Engine.LightComponentBase|GetIntensity (Variables|Default|GetPointLight)) 4e+03
        (:>
          (Rendering|Components|Light|SetIntensity (Variables|Default|GetPointLight) (Math|Float|Lerp (Variables|Default|GetMaxIntensity) (Variables|Default|GetMinIntensity) _intensity)))))))

(event EventTick
  (params (DeltaSeconds :type Float%20%28single-precision%29))
  (bind _pointlight (Variables|Default|GetPointLight))
  (if (Variables|Default|GetEnabled)
    ;[1 1 1] turnb on the light with animation
    (Math|Float|CompareFloat (Variables|/Script/Engine.LightComponentBase|GetIntensity _pointlight) 4e+03
      (:<
        (Rendering|Components|Light|SetIntensity _pointlight (+ (Variables|/Script/Engine.LightComponentBase|GetIntensity _pointlight) 1e+02))))))

(event Collision|EventActorBeginOverlap
  (params (OtherActor :type Actor%20Object%20Reference))
  ;[0.5493 1 0.577] checking overlap with player
  (bind _asbp_player (Utilities|Casting|CastToBP_Player OtherActor))
  (if (Variables|/Game/BluePrint/Players_BP/BP_Player.BP_Player_C|GetLightIsOn _asbp_player)
    (Variables|Default|SetoverlapPlayer true)))

(event Collision|EventActorEndOverlap
  (params (OtherActor :type Actor%20Object%20Reference))
  ;[0.5493 1 0.577] checking overlap with player
  (Utilities|Casting|CastToBP_Player OtherActor)
  (Variables|Default|SetoverlapPlayer false))

(fn ConstructionScript
  (CallFunction|SetEnabled (Variables|Default|GetEnabled)))

(fn SetEnabled
  (params (Enabled :type Boolean))
  (bind _pointlight (Variables|Default|GetPointLight))
  (bind _output_get (Variables|Default|SetEnabled Enabled))
  (Rendering|SetVisibility _pointlight _output_get false)
  (if _output_get
    (Rendering|Components|Light|SetIntensity _pointlight 1.0)
    (else
      (Rendering|Components|Light|SetIntensity _pointlight 0.0)))
  (Rendering|SetVisibility (Variables|Default|GetPS_CandlesFlame) _output_get false)
  (Rendering|SetCastShadow (Variables|Debug|GetStaticMeshComponent) (not _output_get))
  (if _output_get
    (bind _asbp_player (Utilities|Casting|CastToBP_Player (Game|Player|GetPlayerPawn 0))
      (:then
        (Variables|Default|SetCurTimer (Variables|/Game/BluePrint/Players_BP/BP_Player.BP_Player_C|GetMaxTimerCandle _asbp_player)))
      (:CastFailed
        _)))
  (return))

(fn Disable
  (Variables|Default|SetCanBeEnable false)
  (return))